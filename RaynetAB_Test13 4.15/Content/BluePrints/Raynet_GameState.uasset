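; Game state for a two-sided Raynet match that tracks the phase, both sides' pawn arrangements, a move stack and the win result.
; Server-prefixed events store the offensive or defensive arrangement, append moves and record the enemy win state, advancing the State enum for setup and victory.
; Confirmation uses a flag so the phase advances only on the second confirm.
; BeginPlay flags authority; Confirm_SetPawn is an empty stub.
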(event Custom|Server_Move
  (params (Move :type Move%20Structure))
  (Utilities|Array|Add (Variables|Default|GetMoveStack) Move))

(event Custom|Server_SetPawn_Arrangement
  (params (Offensive :type Boolean) (Setting :type Array%20of%20ShowType%20Enums))
  (if Offensive
    (Variables|Default|SetSetPawn_Arrangement_Offensive Setting)
    (else
      (Variables|Default|SetSetPawn_Arrangement_Defensive Setting)))
  (if (Utilities|Enum|Equal(Enum) (Variables|Default|GetState) "NewEnumerator1")
    (Variables|Default|SetState "NewEnumerator4")
    (else
      (Variables|Default|SetState "NewEnumerator5"))))

(event Custom|Server_Confirm
  (if (Variables|Default|GetFlag_OnesideFinished)
    (Variables|Default|SetState "NewEnumerator2")
    (else
      (Variables|Default|SetFlag_OnesideFinished true))))

(event Custom|Server_Win
  (params (EnemyWinState :type Boolean))
  (Variables|Default|SetEnemyWinState EnemyWinState)
  (Variables|Default|SetState "NewEnumerator3"))

(event EventBeginPlay
  (Networking|SwitchHasAuthority
    (:Authority
      (Variables|Default|SetAuthority true))))

(fn ConstructionScript)

(fn ConfirmSetPawn)