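; Raynet game mode that assigns server or client roles to player controllers as they log in.
; On PostLogin, the first player's Raynet_PlayerController is flagged to act as server.
; When the second player joins, it advances the Raynet_GameState state and clears that player's server flag.
; Logins beyond two players receive no handling.
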(event EventPostLogin
  (params (NewPlayer :type Player%20Controller%20Object%20Reference))
  (if (== (Variables|Default|GetNumPlayers) 2)
    (bind _asraynet_game_state (Utilities|Casting|CastToRaynet_GameState (Game|GetGameState)))
    (Variables|/Game/BluePrints/Raynet_GameState.Raynet_GameState_C|SetState _asraynet_game_state "NewEnumerator6")
    (bind _asraynet_player_controller (Utilities|Casting|CastToRaynet_PlayerController NewPlayer))
    (Variables|/Game/BluePrints/Raynet_PlayerController.Raynet_PlayerController_C|SetThisPlayerActAsServer _asraynet_player_controller false)
    (elif (not (> (Variables|Default|GetNumPlayers) 2))
      (bind _asraynet_player_controller_2 (Utilities|Casting|CastToRaynet_PlayerController NewPlayer))
      (Variables|/Game/BluePrints/Raynet_PlayerController.Raynet_PlayerController_C|SetThisPlayerActAsServer _asraynet_player_controller_2 true))))

(fn ConstructionScript)