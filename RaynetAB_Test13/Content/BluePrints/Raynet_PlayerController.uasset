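; Player controller for the Raynet game that relays player actions to the game state.
; Its events cover pawn arrangement, confirmation, moves and win reporting.
; Each casts the game state to Raynet_GameState and forwards its arguments to the matching server function there, holding no game logic itself.
; The Server_ naming suggests these are RPCs giving clients a route to server-side match logic.
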(event Custom|Server_Move
  (params (Move :type Move%20Structure))
  (bind _asraynet_game_state (Utilities|Casting|CastToRaynet_GameState (Game|GetGameState)))
  (Default|ServerMove _asraynet_game_state Move))

(event Custom|Server_SetPawn_Arrangement
  (params (Offensive :type Boolean) (Setting :type Array%20of%20ShowType%20Enums))
  (bind _asraynet_game_state (Utilities|Casting|CastToRaynet_GameState (Game|GetGameState)))
  (Default|ServerSetPawnArrangement _asraynet_game_state Offensive Setting))

(event Custom|Server_Confirm
  (bind _asraynet_game_state (Utilities|Casting|CastToRaynet_GameState (Game|GetGameState)))
  (Default|ServerConfirm _asraynet_game_state))

(event Custom|Server_Win
  (params (EnemyWinState :type Boolean))
  (bind _asraynet_game_state (Utilities|Casting|CastToRaynet_GameState (Game|GetGameState)))
  (Default|ServerWin _asraynet_game_state EnemyWinState))

(event EventBeginPlay)

(fn ConstructionScript)